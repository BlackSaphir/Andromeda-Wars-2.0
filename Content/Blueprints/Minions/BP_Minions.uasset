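; Lane minion Blueprint that takes team- and lane-specific waypoints from the game mode on possession and tags itself with its team.
; Seeing a character without that tag sets the Blackboard enemy key and spawns a homing-target projectile at it, without gating on the computed range check.
; Tick destroys the last projectile once its target is invalid.
; Damage reduces health, destroying the minion at zero.
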(event `self.ReceiveTick`
  (params (DeltaSeconds :type "Float (single-precision)"))
  (`/Engine/EditorBlueprintResources/StandardMacros.IsValid` (`self.ProjectileMinionsTarget`)
    (:`Is Not Valid`
      (`self.K2_DestroyActor` (stale `self.PawnSensing.OnSeePawn` _returnvalue)))))

(event `self.PawnSensing.OnSeePawn`
  (params (Pawn :type "Pawn Object Reference"))
  (bind _ascharacter (cast `Character` Pawn))
  (bind _item (`KismetArrayLibrary.Array_Get` (stale `self.ReceivePossessed` _output_get_2)))
  ;[1 1 1] Spawn/Shoot Projectile
  (if (not (`self.ActorHasTag` _ascharacter _item))
    (`BlackboardComponent.SetValueAsObject` (`AIBlueprintHelperLibrary.GetBlackboard` self) (`self.TargetEnemyKey`) _ascharacter)
    (set `self.bIsInRange` (<= (`self.GetDistanceTo` _ascharacter null) (`self.AttackRange`)))
    (bind _returnvalue (`|SpawnActorFromClass` "/Game/Blueprints/Minions/Projectile_Minion_BP.Projectile_Minion_BP_C" (`KismetMathLibrary.Conv_VectorToTransform` (`SceneComponent.K2_GetComponentLocation` (`self.ShootingPoint`))) "Undefined" "OverrideRootScale" null null _item "0.000000,0.000000,0.000000|0.000000,0.000000,0.000000|1.000000,1.000000,1.000000" self))
    (set `self.ProjectileMinionsTarget` Pawn)
    (set `/Game/Blueprints/Minions/Projectile_Minion_BP.MyTarget` (`KismetArrayLibrary.Array_Get` (`self.K2_GetComponentsByClass` _ascharacter "/Script/Engine.CapsuleComponent")) _returnvalue)))

(event `self.ReceivePossessed`
  (params (NewController :type "Controller Object Reference"))
  ;[1 1 1] Get Waypoints
  (bind _asbp_ch_game_mode (cast `/Game/Blueprints/Charakter/BP_CH_GameMode` (`GameplayStatics.GetGameMode`)))
  (bind _output_get (set `self.Stored Game Mode` _asbp_ch_game_mode))
  (bind _waypoints (`/Game/Blueprints/Charakter/BP_CH_GameMode.GetWaypointsForMinion` _output_get (`self.Team`) (`self.Lane`)))
  (set `self.Waypoints` _waypoints)
  (bind _output_get_2 (set `self.Tags` (`|MakeArray` (`KismetStringLibrary.Conv_StringToName` (`KismetStringLibrary.Conv_IntToString` (`self.Team`)))))))

(event `self.ReceiveAnyDamage`
  (params (Damage :type "Float (single-precision)") (DamageType :type "DamageType Object Reference") (InstigatedBy :type "Controller Object Reference") (DamageCauser :type "Actor Object Reference"))
  ;[1 1 1] Damage
  (set `self.Incoming Damage` Damage)
  (set `self.Health` (- (`self.Health`) (`self.Incoming Damage`)))
  (if (<= (`self.Health`) 0.0)
    (`self.K2_DestroyActor`)))

(fn `UserConstructionScript`)