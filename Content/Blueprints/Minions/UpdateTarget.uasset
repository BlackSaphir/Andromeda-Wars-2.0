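; Behavior tree service that advances minions along their waypoint path.
; On each AI tick, it checks whether the BP_Minions pawn is within a threshold distance of its current waypoint.
; When close enough, it increments the blackboard waypoint index, clamped to the last entry, and writes that waypoint to the target actor key.
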(event `self.ReceiveTickAI`
  (params (OwnerController :type "AIController Object Reference") (ControlledPawn :type "Pawn Object Reference") (DeltaSeconds :type "Float (single-precision)"))
  (bind _returnvalue (`BTFunctionLibrary.GetBlackboardValueAsInt` (`self.CurrentWaypointKey`)))
  (bind _asbp_minions (cast `/Game/Blueprints/Minions/BP_Minions` ControlledPawn))
  (bind _waypoints (`/Game/Blueprints/Minions/BP_Minions.Waypoints` _asbp_minions))
  (bind _item (`KismetArrayLibrary.Array_Get` _waypoints _returnvalue))
  (if (< (`KismetMathLibrary.VSize` (- (`Actor.K2_GetActorLocation` ControlledPawn) (`Actor.K2_GetActorLocation` _item))) (`self.DistanceToUpdateAI`))
    (`BTFunctionLibrary.SetBlackboardValueAsInt` (`self.CurrentWaypointKey`) (`KismetMathLibrary.Min` (+ _returnvalue 1) (`KismetArrayLibrary.Array_LastIndex` _waypoints)))
    ;[1 1 1] Remove Decision to be made in Tree
    (`BTFunctionLibrary.SetBlackboardValueAsObject` (`self.TargetActorKey`) _item)))