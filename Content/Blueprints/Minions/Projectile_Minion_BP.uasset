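; Homing projectile for minions that chases its MyTarget and damages what it hits.
; The homing target is set at BeginPlay and refreshed every Tick while MyTarget is valid.
; On Hit it deals fixed damage to minions lacking its TeamTag and to any BP_CH_Mecha, then destroys itself.
; Friendly minions also destroy it but get no damage value, and the nodes meant to ignore their collision are unwired.
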(event `self.ReceiveBeginPlay`
  (bind _mytarget (`self.MyTarget`))
  (`/Engine/EditorBlueprintResources/StandardMacros.IsValid` _mytarget :!label _label
    (:`Is Valid`
      (set `ProjectileMovementComponent.HomingTargetComponent` _mytarget (`self.ProjectileMovement`)))))

(event `self.ReceiveTick`
  (params (DeltaSeconds :type "Float (single-precision)"))
  (`|ExecutionSequence`
    (:`then_0`
      (goto _label))))

(event `self.ReceiveHit`
  (params (MyComp :type "PrimitiveComponent Object Reference") (Other :type "Actor Object Reference") (OtherComp :type "PrimitiveComponent Object Reference") (bSelfMoved :type Boolean) (HitLocation :type "Vector Structure") (HitNormal :type "Vector Structure") (NormalImpulse :type "Vector Structure") (Hit :type "HitResult Structure (by ref)"))
  ;[1 1 1] Damage
  (`|ExecutionSequence`
    (:`then_0`
      (bind _asbp_minions (cast `/Game/Blueprints/Minions/Minions/BP_Minions` Other))
      (if (not (`self.ActorHasTag` _asbp_minions (`self.TeamTag`)))
        (`GameplayStatics.ApplyDamage` Other 100.0)
        (`self.K2_DestroyActor`)))
    (:`then_1`
      (cast `/Game/Blueprints/Charakter/BP_CH_Mecha` Other)
      (`GameplayStatics.ApplyDamage` Other 100.0)
      (`self.K2_DestroyActor`))
    (:`then_2`
      (bind _asbp_minions_2 (cast `/Game/Blueprints/Minions/Minions/BP_Minions` Other))
      (if (`self.ActorHasTag` _asbp_minions_2 (`self.TeamTag`))
        (`GameplayStatics.ApplyDamage` Other)
        (`self.K2_DestroyActor`)))))

(fn `UserConstructionScript`)