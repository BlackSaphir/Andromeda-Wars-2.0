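; BP_Minions_AIController is the AI controller for minions, starting their behavior tree and seeding its blackboard.
; On possess it runs BT_Minion, then casts the pawn to BP_Minions to copy its ranged flag and attack range into blackboard keys.
; It sets the pawn's first waypoint as the initial move location and target actor, with the waypoint index at zero.
; A failed cast only prints a debug message.
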(event `self.OnPossess`
  (params (PossessedPawn :type "Pawn Object Reference"))
  (bind _returnvalue (`AIBlueprintHelperLibrary.GetBlackboard` null))
  (`self.RunBehaviorTree` "/Game/Blueprints/Minions/BT_Minion.BT_Minion")
  (bind _asbp_minions (cast `/Game/Blueprints/Minions/BP_Minions` PossessedPawn)
    (:`then`
      (`BlackboardComponent.SetValueAsBool` _returnvalue (`self.bIsRangedKey`) (`/Game/Blueprints/Minions/BP_Minions.bIsRanged` _asbp_minions))
      (`BlackboardComponent.SetValueAsFloat` _returnvalue (`self.AttackRangeKey`) (`/Game/Blueprints/Minions/BP_Minions.AttackRange` _asbp_minions))
      (bind _item (`KismetArrayLibrary.Array_Get` (`/Game/Blueprints/Minions/BP_Minions.Waypoints` _asbp_minions)))
      (`BlackboardComponent.SetValueAsVector` _returnvalue (`self.MoveToLocationKey`) (`self.K2_GetActorLocation` _item))
      (`BlackboardComponent.SetValueAsInt` _returnvalue (`self.CurrentWaypoint Key`) 0)
      (`BlackboardComponent.SetValueAsObject` _returnvalue (`self.TargetActorKey`) _item))
    (:`CastFailed`
      (`KismetSystemLibrary.PrintString` "Has Failed"))))

(fn `UserConstructionScript`)