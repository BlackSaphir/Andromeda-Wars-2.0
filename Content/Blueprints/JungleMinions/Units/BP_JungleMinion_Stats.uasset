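; Jungle minion unit with health that attacks BP_CH_Mecha characters entering its attack radius.
; On overlap it spawns one projectile at its billboard, targeting the mecha's capsule; leaving Radius clears the in-range flag.
; Damage from other instigators lowers health and destroys the minion at zero.
; The respawn is unfinished: a delayed timer set after destruction calls an empty SpawnActor event, and the offset uses SpawnPoint's relative location.
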(event `self.ReceiveAnyDamage`
  (params (Damage :type "Float (single-precision)") (DamageType :type "DamageType Object Reference") (InstigatedBy :type "Controller Object Reference") (DamageCauser :type "Actor Object Reference"))
  (if (not (== InstigatedBy self))
    (set `self.IncomingDmg` (`KismetMathLibrary.FTrunc` Damage))
    (set `self.Health` (- (`self.Health`) (`self.IncomingDmg`)))
    (if (<= (`self.Health`) 0)
      (`self.K2_DestroyActor`)
      (`KismetSystemLibrary.K2_SetTimerDelegate` (delegate `SpawnActor`) 40.0)
      (`self.K2_AddActorWorldOffset` (`SceneComponent.RelativeLocation` (`self.SpawnPoint`))))))

(event `SpawnActor`)

(event `self.AttackRadius.OnComponentBeginOverlap`
  (params (OverlappedComponent :type "PrimitiveComponent Object Reference") (OtherActor :type "Actor Object Reference") (OtherComp :type "PrimitiveComponent Object Reference") (OtherBodyIndex :type Integer) (bFromSweep :type Boolean) (SweepResult :type "HitResult Structure (by ref)"))
  (bind _asbp_ch_mecha (cast `/Game/Blueprints/Charakter/BP_CH_Mecha` OtherActor))
  (set `self.IsInRange` true)
  (set `self.Target` (`Character.CapsuleComponent` _asbp_ch_mecha))
  (if (`self.IsInRange`)
    (bind _returnvalue (`|SpawnActorFromClass` "/Game/Blueprints/Turret/Projectile.Projectile_C" (`KismetMathLibrary.MakeTransform` (`SceneComponent.K2_GetComponentLocation` (`self.Billboard`))) "DontSpawnIfColliding" "OverrideRootScale"))
    (set `/Game/Blueprints/Turret/Projectile.ProjectileTarget` (`self.Target`) _returnvalue)))

(event `self.Radius.OnComponentEndOverlap`
  (params (OverlappedComponent :type "PrimitiveComponent Object Reference") (OtherActor :type "Actor Object Reference") (OtherComp :type "PrimitiveComponent Object Reference") (OtherBodyIndex :type Integer))
  (cast `/Game/Blueprints/Charakter/BP_CH_Mecha` OtherActor)
  (set `self.IsInRange` false))

(event `OnDestroyed_Event_0` :!signature `self.OnDestroyed`
  (params (DestroyedActor :type "Actor Object Reference"))
  (add `self.OnDestroyed` (delegate `OnDestroyed_Event_0`))
  (cast `/Game/Blueprints/Charakter/BP_CH_Mecha` DestroyedActor)
  (set `self.Health` 200))

(fn `UserConstructionScript`)