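; MOBA-style game mode that sets up three-lane waypoint paths and spawns minion waves for two teams.
; BeginPlay sorts waypoints into per-lane arrays, reversed for team 1, served by GetWaypointsForMinion.
; A looping one-second timer drives a DoN that spawns minions at every spawn point, passing team and lane.
; A non-looping SpawnTime timer resets that five-count gate once, if at most 30 minions exist.
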(event `self.ReceiveBeginPlay`
  (bind _waypointcounts (`self.WaypointCounts`))
  (bind _waypointcounts_2 (`self.WaypointCounts`))
  (`|ExecutionSequence`
    (:`then_0`
      (bind _outactors (`GameplayStatics.GetAllActorsOfClass` "/Game/Blueprints/Minions/BP_Waypoint.BP_Waypoint_C"))
      (`KismetArrayLibrary.Array_Clear` _waypointcounts)
      (`KismetArrayLibrary.Array_Resize` _waypointcounts 3)
      ;[1 1 1] Count number of Waypoints in Lane
      (for _array_element _outactors
        (bind _lane (`/Game/Blueprints/Minions/BP_Waypoint.Lane` _array_element))
        (`KismetArrayLibrary.Array_Set` _waypointcounts_2 _lane (+ (`KismetArrayLibrary.Array_Get` _waypointcounts_2 _lane) 1)))
      ;[1 1 1] Setting our Waypoint Arrays
      (for _array_element_2 _outactors
        (bind _lane_2 (`/Game/Blueprints/Minions/BP_Waypoint.Lane` _array_element_2))
        (switch `int` _lane_2
          (:`0`
            (bind _waypointnumber (`/Game/Blueprints/Minions/BP_Waypoint.WaypointNumber` _array_element_2))
            (`KismetArrayLibrary.Array_Set` (`self.Team0Lane0`) _waypointnumber _array_element_2 true)
            (bind _returnvalue (- (- (`KismetArrayLibrary.Array_Get` (`self.WaypointCounts`) _lane_2) 1) _waypointnumber))
            (`KismetArrayLibrary.Array_Set` (`self.Team1Lane0`) _returnvalue _array_element_2 true))
          (:`1`
            (`KismetArrayLibrary.Array_Set` (`self.Team0Lane1`) _waypointnumber _array_element_2 true)
            (`KismetArrayLibrary.Array_Set` (`self.Team1Lane1`) _returnvalue _array_element_2 true))
          (:`2`
            (`KismetArrayLibrary.Array_Set` (`self.Team0Lane2`) _waypointnumber _array_element_2 true)
            (`KismetArrayLibrary.Array_Set` (`self.Team1Lane2`) _returnvalue _array_element_2 true)))))
    (:`then_1`
      (`KismetSystemLibrary.Delay` 1.0)
      (`KismetSystemLibrary.K2_SetTimerDelegate` (delegate `SpawnSubWave`) 1.0 true)
      (`KismetSystemLibrary.K2_SetTimerDelegate` (delegate `SpawnMinionWave`) (`self.SpawnTime`)))
    (:`then_2`
      (bind _outactors_2 (`GameplayStatics.GetAllActorsOfClass` "/Game/Blueprints/Minions/MinionSpawnPoint.MinionSpawnPoint_C"))
      (set `self.MiniosSpawns` _outactors_2))))

(event `SpawnMinionWave`
  (bind _miniosspawns (`self.MiniosSpawns`))
  ;[1 1 1] Spawn
  ;;[1 1 1] How many Minions on Map
  (bind _outactors (`GameplayStatics.GetAllActorsOfClass` "/Game/Blueprints/Minions/BP_Minions.BP_Minions_C"))
  (if (<= (`KismetArrayLibrary.Array_Length` _outactors) 30)
    (goto _label :!via `Reset`)))

(event `SpawnSubWave`
  (bind _miniosspawns (`self.MiniosSpawns`))
  ;[1 1 1] Spawn
  (`/Engine/EditorBlueprintResources/StandardMacros.Do N` 5 :!label _label
    (:`Exit`
      (for _index (range (+ (`KismetArrayLibrary.Array_LastIndex` _miniosspawns) 1))
        (bind _item (`KismetArrayLibrary.Array_Get` _miniosspawns _index))
        (bind (_returnvalue_location _returnvalue_rotation) (`KismetMathLibrary.BreakTransform` (`self.GetTransform` _item)))
        (bind _returnvalue (`|SpawnActorFromClass` "/Game/Blueprints/Minions/BP_Minions.BP_Minions_C" (`KismetMathLibrary.MakeTransform` _returnvalue_location _returnvalue_rotation) "AlwaysSpawn" "OverrideRootScale" null (`/Game/Blueprints/Minions/MinionSpawnPoint.Team` _item) (`/Game/Blueprints/Minions/MinionSpawnPoint.Lane` _item)))
        (`KismetArrayLibrary.Array_Add` (`self.MinonArray`) _returnvalue)))))

(fn `GetWaypointsForMinion`
  (params (Team :type Integer) (Lane :type Integer))
  (returns (Waypoints :type "Array of /Game/Blueprints/Minions/BP_Waypoint Object Reference"))
  (return (select `int` (+ (* Team 3) Lane) :`0` (`self.Team0Lane0`) :`1` (`self.Team0Lane1`) :`2` (`self.Team0Lane2`) :`3` (`self.Team1Lane0`) :`4` (`self.Team1Lane1`) :`5` (`self.Team1Lane2`))))

(fn `UserConstructionScript`)