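; Player controller for click-to-move control of the BP_CH_Mecha character, including attack and E ability input.
; Gates opened while the move or attack input is held drive Tick, which either moves the pawn toward the cursor hit beyond a minimum distance or calls the mecha's DamageUpdate with a debug print.
; E triggers the mecha's EAbility, then an IsJumping flag and Delay lock it out as a cooldown.
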(event `self.ReceiveBeginPlay`)

(event `self.ReceiveTick`
  (params (DeltaSeconds :type "Float (single-precision)"))
  (`|ExecutionSequence`
    (:`then_0`
      ;[1 1 1] Movement
      (`/Engine/EditorBlueprintResources/StandardMacros.Gate` true :!label _label
        (:`Exit`
          (`self.MoveToHitLocation` (`self.GetHitResultUnderCursorByChannel` "TraceTypeQuery1")))))
    (:`then_1`
      (`/Engine/EditorBlueprintResources/StandardMacros.Gate` true :!label _label_2
        (:`Exit`
          (bind _asbp_ch_mecha (cast `/Game/Blueprints/Charakter/BP_CH_Mecha` (`GameplayStatics.GetPlayerCharacter` 0)))
          ;[1 1 1] E
          (`/Game/Blueprints/Charakter/BP_CH_Mecha.Damage Update` _asbp_ch_mecha)
          (`KismetSystemLibrary.PrintString` "Hello"))))))

(event `InputAction|Cursor To World`
  (params (Key :type "Key Structure" :default "AnyKey"))
  ;[1 1 1] Movement
  (:`Pressed`
    (goto _label :!via `Open`))
  (:`Released`
    (goto _label :!via `Close`)))

(event `InputAction|E_Ability`
  (params (Key :type "Key Structure" :default "AnyKey"))
  ;[1 1 1] E
  (:`Pressed`
    (if (not (`self.IsJumping`))
      (set `self.IsJumping` true)
      (bind _asbp_ch_mecha (cast `/Game/Blueprints/Charakter/BP_CH_Mecha` (`GameplayStatics.GetPlayerCharacter` 0)))
      (`/Game/Blueprints/Charakter/BP_CH_Mecha.E_Ability` _asbp_ch_mecha)
      (`KismetSystemLibrary.Delay` 14.0)
      (set `self.IsJumping` false))))

(event `InputAction|Attack Target`
  (params (Key :type "Key Structure" :default "AnyKey"))
  (:`Pressed`
    (goto _label_2 :!via `Open`))
  (:`Released`
    (goto _label_2 :!via `Close`)))

(fn `MoveToHitLocation`
  (params (Hit :type "HitResult Structure"))
  (bind (_bblockinghit _binitialoverlap _time _location) (`GameplayStatics.BreakHitResult` Hit))
  (if (>= (`KismetMathLibrary.VSize` (- (`self.K2_GetActorLocation` (`self.K2_GetPawn`)) _location)) (`self.Min Click Distance`))
    (`NavigationSystem.SimpleMoveToLocation` self _location)))

(fn `UserConstructionScript`)