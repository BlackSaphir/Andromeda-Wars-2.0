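; Inhibitor structure actor with health and defense stats, shown through an Inhibitor_Widget created on BeginPlay.
; A damage event feeds UpdateHealth, meant to subtract defense from damage and destroy the actor at zero health, then refreshes the widget through UIUpdate.
; It also checks two linked Inhibitors' alive state before casting to MotherCore, with nothing after the cast.
; SetAktive sets hidden, collision and tick from one bool.
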(event `self.ReceiveBeginPlay`
  ;[1 1 1] Stats
  (`|ExecutionSequence`
    (:`then_0`
      ;[1 1 1] Set Widget
      (bind _returnvalue (`|CreateWidget` "/Game/Blueprints/Turret/Inhibitor_Widget.Inhibitor_Widget_C"))
      (set `self.Inhibitor Widget` _returnvalue))
    (:`then_1`
      (`|ExecutionSequence`
        (:`then_0`
          (bind _updating (`self.Update Health` 0.0))
          (`self.UI Update` _updating))
        (:`then_1`
          (bind _updating_2 (`self.Update Defends`))
          (`self.UI Update` _updating_2))))))

(event `CustomEvent`
  (params (Damage :type "Float (double-precision)") (DamageType :type "DamageType Object Reference") (InstigatedBy :type "Controller Object Reference") (DamageCauser :type "Actor Object Reference"))
  ;[1 1 1] Take Damage
  (bind _output_get (set `self.incoming Value` Damage))
  (bind _updating (`self.Update Health` _output_get))
  (`self.UI Update` _updating)
  ;[1 1 1] Inhibitor Still Alive?
  (if (<= (`self.Max Health`) (- (`self.Max Health`) (`self.Incoming value`)))
    (bind _asinhibitor (cast `/Game/Blueprints/Turret/Inhibitor` (`self.Actor_In_1`)))
    (if (`/Game/Blueprints/Turret/Inhibitor.IsAlive` _asinhibitor)
      (bind _asinhibitor_2 (cast `/Game/Blueprints/Turret/Inhibitor` (`self.Actor_In_2`)))
      (if (not (`/Game/Blueprints/Turret/Inhibitor.IsAlive` _asinhibitor_2))
        (cast `/Game/Blueprints/Turret/MotherCore` (`self.ActorMother`) :!label _label))
      (else
        (goto _label)))
    (else
      (goto _label))))

(fn `Set Aktive`
  (params (`Enable bool` :type Boolean))
  (`self.SetActorHiddenInGame` `Enable bool`)
  (`self.SetActorEnableCollision` `Enable bool`)
  (`self.SetActorTickEnabled` `Enable bool`))

(fn `UI Update`
  (params (Updating :type "/Game/Blueprints/Turret/StatsEnumturret2 Enum"))
  (bind _current_defends (`self.Current Defends`))
  (bind _inhibitor_widget (`self.Inhibitor Widget`))
  (bind _inhibitor_widget_2 (`self.Inhibitor Widget`))
  (bind _current_health (`self.Current Health`))
  (bind _max_health (`self.Max Health`))
  (switch `/Game/Blueprints/Turret/StatsEnumturret2` Updating
    (:`NewEnumerator0`
      (set `/Game/Blueprints/Turret/Inhibitor_Widget.Update Health` (/ _current_health _max_health) _inhibitor_widget)
      (set `/Game/Blueprints/Turret/Inhibitor_Widget.HealthText2` (`KismetStringLibrary.Concat_StrStr` (`KismetStringLibrary.Concat_StrStr` (`KismetStringLibrary.Conv_IntToString` (`KismetMathLibrary.FFloor` _current_health)) "/") (`KismetStringLibrary.Conv_IntToString` (`KismetMathLibrary.FFloor` _max_health))) _inhibitor_widget))
    (:`NewEnumerator1`
      ;[0.2079 1 0.08891] Defends
      (set `/Game/Blueprints/Turret/Inhibitor_Widget.Update Defends` _current_defends _inhibitor_widget_2)
      (set `/Game/Blueprints/Turret/Inhibitor_Widget.DefendsText2` (`KismetStringLibrary.Conv_IntToString` (`KismetMathLibrary.FFloor` _current_defends)) _inhibitor_widget_2))))

(fn `Update Defends`
  (returns (Updating :type "/Game/Blueprints/Turret/StatsEnumturret2 Enum"))
  (set `self.Current Defends` (+ (`self.Current Defends`) 0.0))
  (return "NewEnumerator0"))

(fn `Update Health`
  (params (Damage :type "Float (double-precision)"))
  (returns (Updating :type "/Game/Blueprints/Turret/StatsEnumturret2 Enum"))
  (if (<= (`self.Current Health`) (`self.Max Health`))
    (set `self.Max Health` (+ (`self.Max Health`) 0.0))
    (set `self.Current Health` 0.0)
    (if (< (`self.Current Defends`) (`self.Incoming Value`))
      (set `self.Tem Damage` (- (`self.Incoming Value`) (`self.Current Defends`)))
      (set `self.Max Health` (`KismetMathLibrary.FClamp` (- (`self.Current Health`) (`self.Tem Damage`)) 0.0 (`self.Max Health`)))
      (if (<= (`self.Current Health`) 0.0)
        (`self.K2_DestroyActor`)
        (return "NewEnumerator0")
        (else
          (return "NewEnumerator0")))
      (else
        (return "NewEnumerator0")))
    (else
      (return "NewEnumerator0"))))

(fn `UserConstructionScript`)