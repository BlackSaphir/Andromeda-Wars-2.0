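; Turret actor that fires projectiles at minions and mechas entering its PissOfRadius and shows its stats on the HUD at BeginPlay.
; Overlap sets the target and, via a DoOnce, starts a looping Fire timer that spawns projectiles aimed at it.
; Leaving GTFO_Radius clears the timer with a zero-time call and resets the DoOnce.
; Health is clamped to zero on damage, so any hit destroys the turret.
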(event `self.ReceiveBeginPlay`
  (bind _asbp_hud (cast `/Game/Blueprints/Charakter/BP_HUD` (`PlayerController.GetHUD` (`GameplayStatics.GetPlayerController` 0))))
  (bind _turret_widgetref (`/Game/Blueprints/Charakter/BP_HUD.Turret Widgetref` _asbp_hud))
  (`TextBlock.SetText` (`/Game/Blueprints/Turret/Turret_Widget.UpdateSpeed` _turret_widgetref) (`KismetTextLibrary.Conv_DoubleToText` (`self.AntkSpeed`) "HalfToEven"))
  (`TextBlock.SetText` (`/Game/Blueprints/Turret/Turret_Widget.UpdateDef` _turret_widgetref) (`KismetTextLibrary.Conv_IntToText` (`self.Armor`)))
  (`TextBlock.SetText` (`/Game/Blueprints/Turret/Turret_Widget.UpdateDmg` _turret_widgetref) (`KismetTextLibrary.Conv_IntToText` (`self.Damage`)))
  (`TextBlock.SetText` (`/Game/Blueprints/Turret/Turret_Widget.Updaterange` _turret_widgetref) (`KismetTextLibrary.Conv_IntToText` (`self.Range`)))
  (`TextBlock.SetText` (`/Game/Blueprints/Turret/Turret_Widget.UpdateHealth` _turret_widgetref) (`KismetTextLibrary.Conv_IntToText` (`self.Health`))))

(event `self.PissOfRadius.OnComponentBeginOverlap`
  (params (OverlappedComponent :type "PrimitiveComponent Object Reference") (OtherActor :type "Actor Object Reference") (OtherComp :type "PrimitiveComponent Object Reference") (OtherBodyIndex :type Integer) (bFromSweep :type Boolean) (SweepResult :type "HitResult Structure (by ref)"))
  (`|ExecutionSequence`
    (:`then_0`
      (bind _asbp_minions (cast `/Game/Blueprints/Minions/BP_Minions` OtherActor))
      (set `self.BIsInRange` false)
      (set `self.Target` (`Character.CapsuleComponent` _asbp_minions)))
    (:`then_1`
      (bind _asbp_ch_mecha (cast `/Game/Blueprints/Charakter/BP_CH_Mecha` OtherActor))
      (set `self.BIsInRange` false)
      (set `self.Target` (`Character.CapsuleComponent` _asbp_ch_mecha))))
  (`/Engine/EditorBlueprintResources/StandardMacros.DoOnce` false :!label _label
    (:`Completed`
      (`KismetSystemLibrary.K2_SetTimerDelegate` (delegate `Fire`) 0.1 true)
      (bind _returnvalue (`|SpawnActorFromClass` "/Game/Blueprints/Turret/Projectile.Projectile_C" (`KismetMathLibrary.Conv_VectorToTransform` (`SceneComponent.K2_GetComponentLocation` (`self.Billboard`))) "Undefined" "OverrideRootScale" :!label _label_2))
      (set `/Game/Blueprints/Turret/Projectile.ProjectileTarget` (`self.Target`) _returnvalue))))

(event `Fire`
  (goto _label_2))

(event `self.GTFO_Radius.OnComponentEndOverlap`
  (params (OverlappedComponent :type "PrimitiveComponent Object Reference") (OtherActor :type "Actor Object Reference") (OtherComp :type "PrimitiveComponent Object Reference") (OtherBodyIndex :type Integer))
  (`|ExecutionSequence`
    (:`then_0`
      (cast `/Game/Blueprints/Minions/BP_Minions` OtherActor)
      (set `self.BIsInRange` false))
    (:`then_1`
      (cast `/Game/Blueprints/Charakter/BP_CH_Mecha` OtherActor)
      (set `self.BIsInRange` false)))
  (`KismetSystemLibrary.K2_SetTimerDelegate` (delegate `Fire`) 0.0)
  (goto _label :!via `Reset`))

(event `self.ReceiveAnyDamage`
  (params (Damage :type "Float (single-precision)") (DamageType :type "DamageType Object Reference") (InstigatedBy :type "Controller Object Reference") (DamageCauser :type "Actor Object Reference"))
  (set `self.incoming Value` (`KismetMathLibrary.FTrunc` Damage))
  (set `self.Health` (`KismetMathLibrary.Clamp` (- (`self.Health`) (`self.incoming Value`))))
  (if (<= (`self.Health`) 0)
    (`self.K2_DestroyActor`)))

(event `Team`
  (bind _outactors (`GameplayStatics.GetAllActorsOfClass` "/Game/Blueprints/Turret/Turret.Turret_C"))
  (for _ _outactors
    (if (== (`self.MyTeam`) 0)
      (set `self.MyTeam` 2)
      (else
        (set `self.MyTeam` 1)))))

(fn `UserConstructionScript`)