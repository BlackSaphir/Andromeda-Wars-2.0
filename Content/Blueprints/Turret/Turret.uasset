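; Turret actor that shoots projectiles at BP_CH_Mecha characters and shows its stats in a HUD widget.
; Radius overlap targets the mecha's capsule and, gated by a DoOnce that resets on leaving the outer radius, spawns a projectile at the billboard.
; Collapsed nodes write speed, armor, damage, range and health to the widget.
; Damage sets Health to damage minus Health, destroying the turret when Health is already depleted.
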(event `self.ReceiveBeginPlay`
  (bind _asbp_hud (cast `/Game/Blueprints/Charakter/BP_HUD` (`PlayerController.GetHUD` (`GameplayStatics.GetPlayerController` 0))))
  (bind _turret_widgetref (`/Game/Blueprints/Charakter/BP_HUD.Turret Widgetref` _asbp_hud))
  (`TextBlock.SetText` (`/Game/Blueprints/Turret/Turret_Widget.UpdateSpeed` _turret_widgetref) (`KismetTextLibrary.Conv_DoubleToText` (`self.AntkSpeed`) "HalfToEven"))
  (`TextBlock.SetText` (`/Game/Blueprints/Turret/Turret_Widget.UpdateDef` _turret_widgetref) (`KismetTextLibrary.Conv_IntToText` (`self.Armor`)))
  (`TextBlock.SetText` (`/Game/Blueprints/Turret/Turret_Widget.UpdateDmg` _turret_widgetref) (`KismetTextLibrary.Conv_IntToText` (`self.Damage`)))
  (`TextBlock.SetText` (`/Game/Blueprints/Turret/Turret_Widget.Updaterange` _turret_widgetref) (`KismetTextLibrary.Conv_IntToText` (`self.Range`)))
  (`TextBlock.SetText` (`/Game/Blueprints/Turret/Turret_Widget.UpdateHealth` _turret_widgetref) (`KismetTextLibrary.Conv_IntToText` (`self.Health`))))

(event `self.PissOfRadius.OnComponentBeginOverlap`
  (params (OverlappedComponent :type "PrimitiveComponent Object Reference") (OtherActor :type "Actor Object Reference") (OtherComp :type "PrimitiveComponent Object Reference") (OtherBodyIndex :type Integer) (bFromSweep :type Boolean) (SweepResult :type "HitResult Structure (by ref)"))
  (bind _asbp_ch_mecha (cast `/Game/Blueprints/Charakter/BP_CH_Mecha` OtherActor))
  (set `self.BIsInRange` false)
  (set `self.Target` (`Character.CapsuleComponent` _asbp_ch_mecha))
  (`/Engine/EditorBlueprintResources/StandardMacros.DoOnce` false :!label _label
    (:`Completed`
      (`KismetSystemLibrary.K2_SetTimerDelegate` (delegate `Fire`))
      (bind _returnvalue (`|SpawnActorFromClass` "/Game/Blueprints/Turret/Projectile.Projectile_C" (`KismetMathLibrary.Conv_VectorToTransform` (`SceneComponent.K2_GetComponentLocation` (`self.Billboard`))) "Undefined" "OverrideRootScale" :!label _label_2))
      (set `/Game/Blueprints/Turret/Projectile.ProjectileTarget` (`self.Target`) _returnvalue))))

(event `self.GTFO_Radius.OnComponentEndOverlap`
  (params (OverlappedComponent :type "PrimitiveComponent Object Reference") (OtherActor :type "Actor Object Reference") (OtherComp :type "PrimitiveComponent Object Reference") (OtherBodyIndex :type Integer))
  (cast `/Game/Blueprints/Charakter/BP_CH_Mecha` OtherActor)
  (set `self.BIsInRange` false)
  (`KismetSystemLibrary.K2_SetTimerDelegate` (delegate `Fire`))
  (goto _label :!via `Reset`))

(event `Fire`
  (goto _label_2))

(event `self.ReceiveAnyDamage`
  (params (Damage :type "Float (single-precision)") (DamageType :type "DamageType Object Reference") (InstigatedBy :type "Controller Object Reference") (DamageCauser :type "Actor Object Reference"))
  (bind _health (`self.Health`))
  (if (<= _health 0)
    (`self.K2_DestroyActor`)
    (else
      (set `self.Health` (`KismetMathLibrary.FFloor` (- Damage (`KismetMathLibrary.Conv_IntToDouble` _health)))))))

(event `CheckDeath`
  (if (<= (`self.Health`) 0)
    (cast `/Game/Blueprints/Turret/Turret` (`self.GetOwner`))
    (`self.K2_DestroyActor`)))

(fn `UserConstructionScript`)