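; MotherCore is a turret core that repeatedly fires targeted projectiles at a BP_CH_Mecha entering its radius, stopping when it leaves the outer radius.
; FireRadius and SuperNova overlaps apply radial damage; their timer events are empty.
; A damage event clamps health to zero, destroying the actor; a three-Inhibitor check also jumps there if one is dead.
; Turret widget stats come via the HUD, mostly zero placeholders except Armor.
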(event `self.PissOfRadius.OnComponentBeginOverlap`
  (params (OverlappedComponent :type "PrimitiveComponent Object Reference") (OtherActor :type "Actor Object Reference") (OtherComp :type "PrimitiveComponent Object Reference") (OtherBodyIndex :type Integer) (bFromSweep :type Boolean) (SweepResult :type "HitResult Structure (by ref)"))
  (bind _asbp_ch_mecha (cast `/Game/Blueprints/Charakter/BP_CH_Mecha` OtherActor))
  (set `self.BIsInRange` false)
  (set `self.Target` (`Character.CapsuleComponent` _asbp_ch_mecha))
  (`/Engine/EditorBlueprintResources/StandardMacros.DoOnce` false :!label _label
    (:`Completed`
      (`KismetSystemLibrary.K2_SetTimerDelegate` (delegate `Fire`) 0.6 true)
      (bind _returnvalue (`|SpawnActorFromClass` "/Game/Blueprints/Turret/Projectile.Projectile_C" (`KismetMathLibrary.Conv_VectorToTransform` (`SceneComponent.K2_GetComponentLocation` (`self.Billboard`))) "Undefined" "OverrideRootScale" :!label _label_2))
      (set `/Game/Blueprints/Turret/Projectile.ProjectileTarget` (`self.Target`) _returnvalue))))

(event `self.GTFO_Radius.OnComponentEndOverlap`
  (params (OverlappedComponent :type "PrimitiveComponent Object Reference") (OtherActor :type "Actor Object Reference") (OtherComp :type "PrimitiveComponent Object Reference") (OtherBodyIndex :type Integer))
  (cast `/Game/Blueprints/Charakter/BP_CH_Mecha` OtherActor)
  (set `self.BIsInRange` false)
  (`KismetSystemLibrary.K2_SetTimerDelegate` (delegate `Fire`))
  (goto _label :!via `Reset`))

(event `Fire`
  (goto _label_2))

(event `self.ReceiveBeginPlay`
  (bind _asbp_hud (cast `/Game/Blueprints/Charakter/BP_HUD` (`PlayerController.GetHUD` (`GameplayStatics.GetPlayerController` 0))))
  (bind _turret_widgetref (`/Game/Blueprints/Charakter/BP_HUD.Turret Widgetref` _asbp_hud))
  (`TextBlock.SetText` (`/Game/Blueprints/Turret/Turret_Widget.UpdateSpeed` _turret_widgetref) (`KismetTextLibrary.Conv_DoubleToText` 0.0 "HalfToEven"))
  (`TextBlock.SetText` (`/Game/Blueprints/Turret/Turret_Widget.UpdateDef` _turret_widgetref) (`KismetTextLibrary.Conv_IntToText` (`self.Armor`)))
  (`TextBlock.SetText` (`/Game/Blueprints/Turret/Turret_Widget.UpdateDmg` _turret_widgetref) (`KismetTextLibrary.Conv_IntToText` 0))
  (`TextBlock.SetText` (`/Game/Blueprints/Turret/Turret_Widget.Updaterange` _turret_widgetref) (`KismetTextLibrary.Conv_IntToText` 0))
  (`TextBlock.SetText` (`/Game/Blueprints/Turret/Turret_Widget.UpdateHealth` _turret_widgetref) (`KismetTextLibrary.Conv_IntToText` 0)))

(event `Fire AoE`)

(event `self.FireRadius.OnComponentBeginOverlap`
  (params (OverlappedComponent :type "PrimitiveComponent Object Reference") (OtherActor :type "Actor Object Reference") (OtherComp :type "PrimitiveComponent Object Reference") (OtherBodyIndex :type Integer) (bFromSweep :type Boolean) (SweepResult :type "HitResult Structure (by ref)"))
  (bind _fireradius (`self.FireRadius`))
  (`KismetSystemLibrary.K2_SetTimerDelegate` (delegate `Fire AoE`) 0.5)
  (`GameplayStatics.ApplyRadialDamage` 200.0 (`SceneComponent.RelativeLocation` _fireradius) (`SphereComponent.SphereRadius` _fireradius)))

(event `CustomEvent`
  (params (Damage :type "Float (double-precision)") (DamageType :type "DamageType Object Reference") (InstigatedBy :type "Controller Object Reference") (DamageCauser :type "Actor Object Reference"))
  (set `self.Incoming value` (`KismetMathLibrary.FTrunc` Damage) :!label _label_3)
  (set `self.Health` (`KismetMathLibrary.Clamp` (- (`self.Health`) (`self.Incoming value`))))
  (if (<= (`self.Health`) 0)
    (`self.K2_DestroyActor`)))

(event `Inhibitor`
  (bind _asinhibitor (cast `/Game/Blueprints/Turret/Inhibitor` (`self.Actor_In_1`)))
  (if (`/Game/Blueprints/Turret/Inhibitor.IsAlive` _asinhibitor)
    (bind _asinhibitor_2 (cast `/Game/Blueprints/Turret/Inhibitor` (`self.Actor_In_2`)))
    (if (`/Game/Blueprints/Turret/Inhibitor.IsAlive` _asinhibitor_2)
      (bind _asinhibitor_3 (cast `/Game/Blueprints/Turret/Inhibitor` (`self.Actor_In_3`)))
      (if (not (`/Game/Blueprints/Turret/Inhibitor.IsAlive` _asinhibitor_3))
        (goto _label_3))
      (else
        (goto _label_3)))
    (else
      (goto _label_3))))

(event `self.Super Nova.OnComponentBeginOverlap`
  (params (OverlappedComponent :type "PrimitiveComponent Object Reference") (OtherActor :type "Actor Object Reference") (OtherComp :type "PrimitiveComponent Object Reference") (OtherBodyIndex :type Integer) (bFromSweep :type Boolean) (SweepResult :type "HitResult Structure (by ref)"))
  (bind _super_nova (`self.Super Nova`))
  (`KismetSystemLibrary.K2_SetTimerDelegate` (delegate `SuperNova`) 60.0)
  (`GameplayStatics.ApplyRadialDamage` 10000.0 (`SceneComponent.RelativeLocation` _super_nova) (`SphereComponent.SphereRadius` _super_nova)))

(event `SuperNova`)

(fn `UserConstructionScript`)